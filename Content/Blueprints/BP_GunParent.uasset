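; BP_GunParent is a gun Blueprint, named as a parent class, that handles automatic hitscan firing.
; Pulling the trigger fires immediately and starts a looping timer based on FireRate, with a DoOnce blocking repeats until release clears the timer and resets it.
; Each shot line-traces on Visibility from the gun to BP_PlayerController's CrosshairPos, drawing debug lines and printing the hit actor's name without applying damage.
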(event Custom|PullTrigger
  ;[1 1 1] FiringGun
  (Utilities|FlowControl|DoOnce false
    (:Completed
      (CallFunction|Fire)
      (Utilities|Time|SetTimerbyFunctionName 0 "Fire" (/ 1.0 (Variables|Default|GetFireRate)) true))))

(event Custom|ReleaseTrigger
  ;[1 1 1] FiringGun
  (Utilities|Time|ClearTimerbyFunctionName 0 "Fire")
  (Utilities|FlowControl|DoOnce false) ; enters at Reset
)

(event Custom|Fire
  ;[1 1 1] FiringGun
  (bind _outhit (Collision|LineTraceByChannel (Transformation|GetActorLocation) (Variables|/Game/Blueprints/BP_PlayerController.BP_PlayerController_C|GetCrosshairPos (.AsBP%20Player%20Controller (Utilities|Casting|CastToBP_PlayerController (Game|GetPlayerController 0)))) "TraceTypeQuery1" false 0 "ForDuration"))
  (Development|PrintString (Utilities|GetDisplayName (.HitActor (Collision|BreakHitResult _outhit)))))

(fn ConstructionScript)