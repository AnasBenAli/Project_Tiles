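; Explosive crate actor that detonates after a countdown, damaging and knocking back nearby enemies and setting off neighboring crates.
; Once Detonate is set, Tick recolors and hops the cube, reveals the radius indicator, and lerps its scale toward ReachedSize.
; Near that size, it plays random sounds and particles, damaging EnemyBP actors within a fixed range.
; Crates within ExplosionDistance explode immediately without recursive chaining, and are destroyed.
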(event EventBeginPlay
  (bind _explosiondistance (Variables|Default|GetExplosionDistance))
  (bind _returnvalue (/ _explosiondistance 1e+02))
  (Transformation|SetWorldScale3D (Variables|Default|GetExplosionRadius) (Math|Vector|MakeVector _returnvalue _returnvalue _returnvalue)))

(event Collision|EventActorBeginOverlap
  (params (OtherActor :type Actor%20Object%20Reference)))

(event EventTick
  (params (DeltaSeconds :type Float%20%28single-precision%29))
  (CallFunction|TriggerExplosion DeltaSeconds))

(fn ConstructionScript)

(fn GetNearbyEnnemies
  (params (Distance :type Float%20%28double-precision%29))
  (bind _nearbyennemies (Variables|Default|GetNearbyEnnemies))
  (Utilities|Array|Clear _nearbyennemies)
  (bind _outactors (Actor|GetAllActorsOfClass "/Game/TopDown/Blueprints/EnemyBP.EnemyBP_C"))
  (for _array_element _outactors
    (if (<= (Transformation|GetDistanceTo _array_element) Distance)
      (Utilities|Array|Insert (Variables|Default|GetNearbyEnnemies) _array_element)))
  (for _array_element_2 _nearbyennemies
    (Development|PrintString (Utilities|GetDisplayName _array_element_2))))

(fn DamageNearbyEnnemies
  (CallFunction|GetNearbyEnnemies 6e+02)
  (for _array_element (Variables|Default|GetNearbyEnnemies)
    (bind _asenemy_bp (Utilities|Casting|CastToEnemyBP _array_element))
    (Default|PushAwayfromLocation _asenemy_bp (Math|Conversions|ToTransform(Vector) (Transformation|GetActorLocation)) (Variables|Default|GetKnockback%20Force%20Magnitude))
    (Default|DealDamage _asenemy_bp (Variables|Default|GetDamage))))

(fn GetNearbyCrates
  (params (Distance :type Float%20%28double-precision%29))
  (bind _nearbycrates (Variables|Default|GetNearbyCrates))
  (Utilities|Array|Clear _nearbycrates)
  (bind _outactors (Actor|GetAllActorsOfClass "ExplosiveCrate_BP_C"))
  (for _array_element _outactors
    (if (<= (Transformation|GetDistanceTo _array_element) Distance)
      (Utilities|Array|Insert (Variables|Default|GetNearbyCrates) _array_element)))
  (Utilities|Array|RemoveItem _nearbycrates self))

(fn TriggerExplosion
  (params (DeltaTime :type Float%20%28double-precision%29))
  (bind _cube (Variables|Default|GetCube))
  (if (Variables|Default|GetDetonate)
    (Utilities|InitialTrigger _cube
      (:then
        _)
      (:else
        _))
    (Transformation|SetRelativeScale3D _cube (Math|Vector|Lerp(Vector) (Variables|/Script/Engine.SceneComponent|GetRelativeScale3D (Variables|Default|GetCube)) (Variables|Default|GetReachedSize) (/ DeltaTime (Variables|Default|GetCountdown))))
    (if (>= (.X (Class|KismetMathLibrary|BreakVector3f (Variables|/Script/Engine.SceneComponent|GetRelativeScale3D (Variables|Default|GetCube)))) (- (.X (Class|KismetMathLibrary|BreakVector3f (Variables|Default|GetReachedSize))) 0.2))
      (Utilities|InitialExplosion)
      (Utilities|SecondaryExplosions))))

(fn PlayRandomExplosion
  (params (Location :type Vector))
  (Audio|PlaySoundatLocation (Utilities|Array|Get(acopy) (Variables|Default|GetExplosionSounds) (Math|Random|RandomInteger (Utilities|Array|Length (Variables|Default|GetExplosionSounds)))) Location "0, 0, 0" 1.0 1.0 0.0 0 0 0 0))