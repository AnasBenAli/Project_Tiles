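; Enemy character that spawns at a randomly enlarged mesh size and shoves the nearby player away, gated by a cooldown flag on the player.
; DealDamage lowers health, updates the health widget and, if aggression is enabled, raises walk speed more as health drops, destroying the actor at zero.
; EndPlay increments the WaveManager's destroyed count and, when not falling, randomly spawns an explosive crate.
; It also provides ragdoll and self-knockback functions.
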(event EventBeginPlay
  (for _index (range 0 (Math|Random|RandomInteger 5))
    (CallFunction|IncreaseSize)))

(event EventEndPlay
  (params (EndPlayReason :type EEndPlayReason%20Enum :default "Destroyed"))
  (Development|PrintString "Enemy Destroyed: ")
  (bind _returnvalue (Actor|GetActorOfClass "/Game/Blueprints/WaveManager.WaveManager_C"))
  (Variables|/Game/Blueprints/WaveManager.WaveManager_C|SetEnemiesDestroyed _returnvalue (+ (Variables|/Game/Blueprints/WaveManager.WaveManager_C|GetEnemiesDestroyed _returnvalue) 1))
  (CallFunction|SpawnCrateatRandom))

(event EventTick
  (params (DeltaSeconds :type Float%20%28single-precision%29))
  (CallFunction|PushPlayer 5e+02))

(fn ConstructionScript)

(fn IncreaseAggression
  (bind _charactermovement (Variables|Character|GetCharacterMovement))
  (if (Variables|Default|GetGetsAggressive)
    (if (< (Variables|/Script/Engine.CharacterMovementComponent|GetMaxWalkSpeed _charactermovement) (Variables|Default|GetMaxWalkSpeed))
      (Variables|/Script/Engine.CharacterMovementComponent|SetMaxWalkSpeed _charactermovement (+ (Variables|/Script/Engine.CharacterMovementComponent|GetMaxWalkSpeed _charactermovement) (* (* (/ 1.0 (Variables|Default|GetHealth)) 0.5) (Variables|Default|GetSpeedIncrease)))))))

(fn IncreaseSize
  (bind _mesh (Variables|Character|GetMesh))
  (bind _returnvalue (Transformation|GetWorldScale _mesh))
  (if (< (.X (Class|KismetMathLibrary|BreakVector3f _returnvalue)) (Variables|Default|GetMaxScaleSize))
    (Transformation|SetWorldScale3D (Variables|Character|GetMesh) (+ _returnvalue (Math|Vector|MakeVector 0.2 0.2 0.2)))))

(fn PushSelffromLocation
  (params (Location :type Transform) (Force :type Float%20%28double-precision%29))
  (bind _ascharacter (Utilities|Casting|CastToCharacter self))
  (Character|LaunchCharacter _ascharacter (* (Math|Vector|GetUnitDirection(Vector) (Math|Transform|TransformLocation Location "0, 0, 0") (Transformation|GetActorLocation _ascharacter)) Force) false false))

(fn DealDamage
  (params (Amount :type Float%20%28double-precision%29))
  (bind _output_get (Variables|Default|SetHealth (- (Variables|Default|GetHealth) Amount)))
  (if (<= (Variables|Default|GetHealth) 0.0)
    (Actor|DestroyActor)
    (else
      (bind _asenemy_uibp (Utilities|Casting|CastToEnemyUIBP (UserInterface|GetUserWidgetObject (Variables|Default|GetWidget))))
      (Variables|/Game/Blueprints/EnemyUIBP.EnemyUIBP_C|SetHealthValue _asenemy_uibp _output_get)
      (CallFunction|IncreaseAggression)
      (Development|PrintString (Utilities|String|ToString(Float) _output_get)))))

(fn SpawnCrateatRandom
  (if (not (AI|Components|NavMovement|IsFalling (Variables|Character|GetCharacterMovement)))
    (if (> (Math|Random|RandomInteger 10) 6)
      (Game|SpawnActorfromClass "/Game/Blueprints/ExplosiveCrate_BP.ExplosiveCrate_BP_C" (Math|Conversions|ToTransform(Vector) (Transformation|GetActorLocation)) "Undefined" 0 0)
      (Effects|SpawnEmitteratLocation "/Game/InfinityBladeEffects/Effects/FX_Ability/Summon/P_Summon_Child_Startup.P_Summon_Child_Startup" (Transformation|GetActorLocation) "0, 0, 0" "2.000000,2.000000,2.000000"))))

(fn Ragdoll
  (Physics|SetSimulatePhysics (Variables|Character|GetMesh) true)
  (Pawn|Components|CharacterMovement|DisableMovement (Variables|Character|GetCharacterMovement)))

(fn PushPlayer
  (params (Force :type Float%20%28double-precision%29))
  (bind _returnvalue (Transformation|GetActorLocation))
  (bind _returnvalue_2 (Actor|GetActorOfClass "/Game/Blueprints/BP_ThirdPersonCharacter.BP_ThirdPersonCharacter_C"))
  (if (not (Variables|/Game/Blueprints/BP_ThirdPersonCharacter.BP_ThirdPersonCharacter_C|GetOnPushCooldown _returnvalue_2))
    (if (<= (Math|Vector|Distance(Vector) _returnvalue (Transformation|GetActorLocation _returnvalue_2)) 3e+02)
      (bind _ascharacter (Utilities|Casting|CastToCharacter _returnvalue_2))
      (Character|LaunchCharacter _ascharacter (* (Math|Vector|GetUnitDirection(Vector) _returnvalue (Transformation|GetActorLocation _ascharacter)) Force) false false)
      (Variables|/Game/Blueprints/BP_ThirdPersonCharacter.BP_ThirdPersonCharacter_C|SetOnPushCooldown _returnvalue_2 true))))