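; Shrinking arena platform that collapses and spawns its own replacement while tracking destroyed platforms in the game mode.
; Once the game starts, looping timers alternate shrink and pause phases until scale hits a threshold derived from initial size.
; Collapse pauses WaveManager spawning, shakes the camera, delays destruction, and moves in a new offset platform.
; Replacements glide to WaveManager's initial platform location, then re-enable spawning; EndPlay emits a blast effect.
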(event Custom|PlatformShrinking
  (bind _returnvalue (Transformation|GetActorScale3D))
  (bind _collapsingthreshold (Variables|Default|GetCollapsingThreshold))
  ;[1 0 0.02461] ShrinkingEvent
  (Transformation|SetActorScale3D (- _returnvalue (Variables|Default|GetShrinkingMagnitude)))
  (if (Utilities|Operators|EqualEqual _returnvalue (Math|Vector|MakeVector (.x _collapsingthreshold) (.y _collapsingthreshold) (.z _collapsingthreshold)) 0.0001)
    (Utilities|Time|ClearTimerbyFunctionName 0 "PlatformShrinking")
    (CallFunction|PlatformCollapsing)))

(event Custom|PlatformCollapsing
  ;[0 0.0582 1] CollapsingEvent
  (bind _returnvalue (Actor|GetActorOfClass "/Game/Blueprints/WaveManager.WaveManager_C"))
  (Variables|/Game/Blueprints/WaveManager.WaveManager_C|SetEnableSpawning _returnvalue false)
  (bind _asbp_third_person_game_mode (Utilities|Casting|CastToBP_ThirdPersonGameMode (Game|GetGameMode)))
  (Default|UpdatePlatformsCount _asbp_third_person_game_mode)
  (Camera|PlayWorldCameraShake "/Game/Blueprints/BP_CameraShake.BP_CameraShake_C" (Transformation|GetActorLocation) 0.0 9e+03)
  (Utilities|FlowControl|Sequence
    (:then_0
      (Utilities|FlowControl|Delay 4.0)
      (Actor|DestroyActor))
    (:then_1
      (bind _returnvalue_2 (Game|SpawnActorfromClass "BP_Platform_C" (Math|Conversions|ToTransform(Vector) (+ (Transformation|GetActorLocation) "4000.000000,0.000000,2000.000000")) "Undefined" 0 0))
      (Variables|Default|SetSpawnedPlatformLocation (Transformation|GetActorLocation _returnvalue_2))
      (bind _vectorlerpfloat (Timeline|PlatformMovement Play)
        (:Update
          (Transformation|SetActorLocation _returnvalue_2 (Math|Vector|Lerp(Vector) (Variables|Default|GetSpawnedPlatformLocation) (- (Variables|Default|GetSpawnedPlatformLocation) (Variables|Default|GetDistanceBetweenPlatforms)) _vectorlerpfloat) false false))))))

(event Custom|ActivatePlatform
  ;[0.09492 1 0] StartingTheShrinking
  (Utilities|Time|SetTimerbyEvent (delegate Custom|PlatformShrinking) (Variables|Default|GetShrinkingSpeed) true))

(event Custom|ShrinkingLoop
  ;[1 0.2599 0.2499] Platform's ShrinkingLoop
  (bind _returnvalue (Actor|GetActorOfClass "/Game/Blueprints/BP_GameManager.BP_GameManager_C"))
  (if (Variables|/Game/Blueprints/BP_GameManager.BP_GameManager_C|GetStartGame _returnvalue)
    (CallFunction|ActivatePlatform)
    (Utilities|FlowControl|Delay (Variables|Default|GetTimeBetweenPhases))
    (CallFunction|DeactivatePlatform)))

(event Custom|DeactivatePlatform
  ;[0.3888 0 1] StoppingTheShrinking
  (Utilities|Time|ClearTimerbyFunctionName 0 "PlatformShrinking"))

(event EventEndPlay
  (params (EndPlayReason :type EEndPlayReason%20Enum :default "Destroyed"))
  (Effects|SpawnEmitteratLocation "/Game/InfinityBladeEffects/Effects/FX_Ability/Defense/P_EnergyBlast_Impact.P_EnergyBlast_Impact" (Transformation|GetActorLocation) "0, 0, 0" "15.000000,15.000000,15.000000"))

(event EventBeginPlay
  (bind _returnvalue (not false))
  (bind _timebetweenphases (Variables|Default|GetTimeBetweenPhases))
  (bind _returnvalue_2 (* _timebetweenphases 2.0))
  ;[0 1 0.6339] BeginPlay
  (Utilities|FlowControl|Sequence
    (:then_0
      ;;[1 0.6998 0] Setting Platform's Initial Scale & Collapsing Threshold
      (bind _output_get (Variables|Default|SetInitialPlatformScale (Transformation|GetActorScale3D)))
      (Variables|Default|SetCollapsingThreshold (* _output_get (Variables|Default|GetShrinkToReach))))
    (:then_1
      (if (> (Variables|/Game/Blueprints/BP_ThirdPersonGameMode.BP_ThirdPersonGameMode_C|GetPlatformsDestroyed (.AsBP%20Third%20Person%20Game%20Mode (Utilities|Casting|CastToBP_ThirdPersonGameMode (Game|GetGameMode)))) 0)
        (Utilities|FlowControl|Delay 5.0)
        (Utilities|Time|SetTimerbyEvent (delegate Custom|ShrinkingLoop) _returnvalue_2 _returnvalue)
        (Variables|Default|SetFinalPlatformPosition (Transformation|GetActorLocation))
        (bind _delta (Timeline|Timeline_0 Play)
          (:Update
            (bind _returnvalue_3 (Actor|GetActorOfClass "/Game/Blueprints/WaveManager.WaveManager_C"))
            (Transformation|SetActorLocation (Math|Vector|Lerp(Vector) (Variables|Default|GetFinalPlatformPosition) (Variables|/Game/Blueprints/WaveManager.WaveManager_C|GetInitialPlatformLocation _returnvalue_3) _delta) false false))
          (:Finished
            (bind _returnvalue_4 (Actor|GetActorOfClass "/Game/Blueprints/WaveManager.WaveManager_C"))
            (Variables|/Game/Blueprints/WaveManager.WaveManager_C|SetEnableSpawning _returnvalue_4 true)))
        (else
          (Utilities|Time|SetTimerbyEvent (delegate Custom|ShrinkingLoop) _returnvalue_2 _returnvalue))))))

(fn ConstructionScript)